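; BP_RandomEnemyGenerator spawns BP_BaseEnemy actors at one of five randomly chosen points in the space shooter.
; Tick drives a randomized Delay as the spawn loop, using a shorter wait range once SecondsProgress reaches a fixed threshold to increase the spawn rate.
; StartCounting resets SecondsProgress and starts a looping timer that increments it every second; nothing in this Blueprint calls it.
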(event Custom|StartCounting
  (Variables|Default|SetSecondsProgress 0.0)
  (Utilities|Time|SetTimerbyEvent (delegate Custom|Count) 1.0 true))

(event Custom|Count
  (Math|Float|IncrementFloat (Variables|Default|GetSecondsProgress)))

(event EventBeginPlay)

(event Collision|EventActorBeginOverlap
  (params (OtherActor :type Actor%20Object%20Reference)))

(event EventTick
  (params (DeltaSeconds :type Float%20%28single-precision%29))
  (bind _returnvalue (Math|Random|RandomIntegerinRange 0 4))
  (bind _point1 (Variables|Default|Getpoint1))
  (bind _point2 (Variables|Default|Getpoint2))
  (bind _point3 (Variables|Default|Getpoint3))
  (bind _point4 (Variables|Default|Getpoint4))
  (bind _point5 (Variables|Default|Getpoint5))
  (bind _array (Utilities|Array|MakeArray _point1 _point2 _point3 _point4 _point5))
  (bind _output (Utilities|Array|Get(acopy) _array _returnvalue))
  (bind _returnvalue_2 (Transformation|GetWorldTransform _output))
  (if (>= (Variables|Default|GetSecondsProgress) 15.0)
    (Utilities|FlowControl|Delay (Math|Conversions|ToFloat(Integer) (Math|Random|RandomIntegerinRange 1 2)))
    (Game|SpawnActorfromClass "/Game/00_Space_shooter/Enemies/BP_BaseEnemy.BP_BaseEnemy_C" _returnvalue_2 "Undefined" "MultiplyWithRoot" 0 0)
    (else
      (Utilities|FlowControl|Delay (Math|Conversions|ToFloat(Integer) (Math|Random|RandomIntegerinRange 2 4)))
      (Game|SpawnActorfromClass "/Game/00_Space_shooter/Enemies/BP_BaseEnemy.BP_BaseEnemy_C" _returnvalue_2 "Undefined" "MultiplyWithRoot" 0 0))))

(fn ConstructionScript)