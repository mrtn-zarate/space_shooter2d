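; Horizontal enemy variant for the space shooter, extending a parent enemy whose BeginPlay, Tick and overlap logic it calls.
; On BeginPlay it sets the shoot delay, points its movement vector along the actor's right axis, negated when IsRight is set, and destroys itself after a fixed lifetime.
; Overlapping an actor tagged "lateral" reassigns IsRight to its existing value, so the direction never flips.
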(event EventBeginPlay
  (bind _returnvalue (Transformation|GetActorRightVector))
  (|CallParentFunction)
  (Variables|Default|SetDelayShoot 2.0)
  (Variables|Default|SetMovementVector (Transformation|GetActorRightVector))
  (if (Variables|Default|GetisRight)
    (Variables|Default|SetMovementVector (* _returnvalue -1))
    (else
      (Variables|Default|SetMovementVector _returnvalue)))
  (Utilities|FlowControl|Delay 4e+01)
  (Actor|DestroyActor))

(event Collision|EventActorBeginOverlap
  (params (OtherActor :type Actor%20Object%20Reference))
  (|CallParentFunction OtherActor)
  (if (Utilities|Array|ContainsItem (Variables|/Script/Engine.Actor|GetTags OtherActor) "lateral")
    (if (Variables|Default|GetisRight)
      (Variables|Default|SetisRight true)
      (else
        (Variables|Default|SetisRight false)))))

(event EventTick
  (params (DeltaSeconds :type Float%20%28single-precision%29))
  (|CallParentFunction DeltaSeconds))

(fn ConstructionScript
  (|CallParentFunction))