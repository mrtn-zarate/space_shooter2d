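; Player pawn for a space shooter, driven by Enhanced Input, with movement and a placeholder fire action.
; On BeginPlay it registers its mapping context with the player controller's input subsystem.
; The movement action caches its 2D value until canceled or completed, and Tick applies it as an unswept, speed-scaled offset, with both axes along the forward vector.
; Fire only prints a debug string.
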(event Input|EnhancedActionEvents|EnhancedInputActionIA_Player_Fire
  (params (ActionValue :type Boolean) (ElapsedSeconds :type Float%20%28double-precision%29) (TriggeredSeconds :type Float%20%28double-precision%29) (InputAction :type Input%20Action%20Object%20Reference :default "/Game/00_Space_shooter/input/IA_Player_Fire.IA_Player_Fire"))
  (:Triggered
    (Development|PrintString "fire")))

(event Input|EnhancedActionEvents|EnhancedInputActionIA_Player_Movement
  (params (ActionValue :type Vector%202D%20Structure) (ElapsedSeconds :type Float%20%28double-precision%29) (TriggeredSeconds :type Float%20%28double-precision%29) (InputAction :type Input%20Action%20Object%20Reference :default "/Game/00_Space_shooter/input/IA_Player_Movement.IA_Player_Movement"))
  (:Triggered
    (Development|PrintString (Utilities|String|ToString(Vector2d) ActionValue))
    (Variables|Default|Setinputsaved ActionValue))
  (:Canceled
    (Variables|Default|Setinputsaved "" :!label _label))
  (:Completed
    (goto _label)))

(event EventBeginPlay
  (bind _asplayer_controller (Utilities|Casting|CastToPlayerController (Pawn|GetController)))
  (Utilities|IsValid (PlayerController|LocalPlayerSubsystems|GetEnhancedInputLocalPlayerSubsystem _asplayer_controller)
    (:Is%20Valid
      (Input|AddMappingContext (PlayerController|LocalPlayerSubsystems|GetEnhancedInputLocalPlayerSubsystem _asplayer_controller) "/Game/00_Space_shooter/input/InputMappingContext.InputMappingContext" 0 "(bIgnoreAllPressedKeysUntilRelease=True,bForceImmediately=False,bNotifyUserSettings=False)"))))

(event Collision|EventActorBeginOverlap
  (params (OtherActor :type Actor%20Object%20Reference)))

(event EventTick
  (params (DeltaSeconds :type Float%20%28single-precision%29))
  (bind _speed (Variables|Default|Getspeed))
  (bind _inputsaved (Variables|Default|Getinputsaved))
  (bind _returnvalue (* DeltaSeconds _speed))
  (Transformation|SetActorLocation (+ (+ (* (Transformation|GetActorForwardVector) (* _returnvalue (.x _inputsaved))) (* (* _returnvalue (.y _inputsaved)) (Transformation|GetActorForwardVector))) (Transformation|GetActorLocation)) false false))

(fn ConstructionScript)