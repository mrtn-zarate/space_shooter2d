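; BP_enemy_horizontal_right is a space shooter enemy variant that sets up horizontal movement along its negative right vector.
; On BeginPlay it runs the parent logic, then overrides the inherited shoot delay and movement vector.
; It adds no movement or firing logic of its own and destroys itself after a fixed 40-second lifetime.
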(event EventBeginPlay
  (|CallParentFunction)
  (Variables|Default|SetDelayShoot 0.9)
  (Variables|Default|SetMovementVector (* (Transformation|GetActorRightVector) -1))
  (Utilities|FlowControl|Delay 4e+01)
  (Actor|DestroyActor))

(event Collision|EventActorBeginOverlap
  (params (OtherActor :type Actor%20Object%20Reference))
  (|CallParentFunction OtherActor) ; This node is disabled and will not be called.\nDrag off pins to build functionality.
)

(event EventTick
  (params (DeltaSeconds :type Float%20%28single-precision%29))
  (|CallParentFunction DeltaSeconds) ; This node is disabled and will not be called.\nDrag off pins to build functionality.
)

(fn ConstructionScript
  (|CallParentFunction))