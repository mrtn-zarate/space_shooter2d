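; Spaceship ammo actor for the space shooter that flies in a straight line as a projectile.
; Tick moves it along its forward vector by Speed scaled by delta time, without sweeping.
; Overlapping a Pawn starts a two-second delay before it destroys itself, and it keeps moving meanwhile.
; The graphs apply no damage and have no other despawn logic.
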(event EventBeginPlay)

(event Collision|EventActorBeginOverlap
  (params (OtherActor :type Actor%20Object%20Reference))
  (Utilities|Casting|CastToPawn OtherActor)
  (Utilities|FlowControl|Delay 2.0)
  (Actor|DestroyActor))

(event EventTick
  (params (DeltaSeconds :type Float%20%28single-precision%29))
  (Transformation|SetActorLocation (+ (Transformation|GetActorLocation) (* (Transformation|GetActorForwardVector) (* DeltaSeconds (Variables|Default|GetSpeed)))) false false))

(fn ConstructionScript)