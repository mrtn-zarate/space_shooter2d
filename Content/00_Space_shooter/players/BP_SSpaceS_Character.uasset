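; Player character for a space shooter, handling movement, firing and lives.
; Enhanced Input drives movement along the actor's axes and firing, which spawns Ammo at FirePoint with a timer-based cooldown.
; Overlapping an Enemy-tagged actor plays an explosion and briefly hides the ship with input disabled, then restores it and calls DamageActor on the player pawn.
; DamageActor decrements Lives, and at zero hides the ship, disables input and notifies the game mode through PlayerDead.
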(event Custom|UpdateFire
  (Variables|Default|SetCanFire true))

(event Custom|DamageActor
  (bind _output_get (Variables|Default|SetLives (- (Variables|Default|GetLives) 1)))
  (if (== _output_get 0)
    (Input|DisableInput (Game|GetPlayerController 0))
    (Rendering|SetActorHiddenInGame true)
    (bind _asgamemodebase (Utilities|Casting|CastTogamemodebase (Game|GetGameMode)))
    (Default|PlayerDead _asgamemodebase)))

(event Input|EnhancedActionEvents|EnhancedInputActionIA_Player_Movement
  (params (ActionValue :type Vector%202D%20Structure) (ElapsedSeconds :type Float%20%28double-precision%29) (TriggeredSeconds :type Float%20%28double-precision%29) (InputAction :type Input%20Action%20Object%20Reference :default "/Game/00_Space_shooter/input/IA_Player_Movement.IA_Player_Movement"))
  (Pawn|Input|AddMovementInput (Transformation|GetActorRightVector) (.x ActionValue) false)
  (Pawn|Input|AddMovementInput (Transformation|GetActorForwardVector) (.y ActionValue) false))

(event Input|EnhancedActionEvents|EnhancedInputActionIA_Player_Fire
  (params (ActionValue :type Boolean) (ElapsedSeconds :type Float%20%28double-precision%29) (TriggeredSeconds :type Float%20%28double-precision%29) (InputAction :type Input%20Action%20Object%20Reference :default "/Game/00_Space_shooter/input/IA_Player_Fire.IA_Player_Fire"))
  (if (Variables|Default|GetCanFire)
    (CallFunction|DoFire)
    (Audio|SpawnSound2D "/Game/00_Space_shooter/Sounds/submachinegun_gunshot_sound.submachinegun_gunshot_sound" 0.15 1.0 0.0 0)
    (Variables|Default|SetCanFire false)
    (Utilities|Time|SetTimerbyEvent (delegate Custom|UpdateFire) (Variables|Default|GetFireDelay))))

(event EventBeginPlay
  (bind _asplayer_controller (Utilities|Casting|CastToPlayerController (Pawn|GetController)))
  (Utilities|IsValid (PlayerController|LocalPlayerSubsystems|GetEnhancedInputLocalPlayerSubsystem _asplayer_controller)
    (:Is%20Valid
      (Input|AddMappingContext (PlayerController|LocalPlayerSubsystems|GetEnhancedInputLocalPlayerSubsystem _asplayer_controller) "/Game/00_Space_shooter/input/InputMappingContext.InputMappingContext" 0 "(bIgnoreAllPressedKeysUntilRelease=True,bForceImmediately=False,bNotifyUserSettings=False)"))))

(event Collision|EventActorBeginOverlap
  (params (OtherActor :type Actor%20Object%20Reference))
  (bind _returnvalue (Game|GetPlayerController 0))
  (if (Utilities|Array|ContainsItem (Variables|/Script/Engine.Actor|GetTags OtherActor) "Enemy")
    (Input|DisableInput _returnvalue)
    (Effects|SpawnEmitteratLocation "/Game/StarterContent/Particles/P_Explosion.P_Explosion" (Transformation|GetActorLocation))
    (Audio|SpawnSound2D "/Game/00_Space_shooter/Sounds/bomb-explosion-dead.bomb-explosion-dead" 0.6 1.0 0.0 0)
    (Rendering|SetActorHiddenInGame true)
    (Utilities|FlowControl|Delay 1.0)
    (Rendering|SetActorHiddenInGame false)
    (Input|EnableInput _returnvalue)
    (bind _asbp_sspace_s_character (Utilities|Casting|CastToBP_SSpaceS_Character (Game|Player|GetPlayerPawn 0)))
    (CallFunction|DamageActor _asbp_sspace_s_character)))

(event EventTick
  (params (DeltaSeconds :type Float%20%28single-precision%29)))

(fn ConstructionScript)

(fn DoFire
  (Game|SpawnActorfromClass (Variables|Default|GetAmmo) (Transformation|GetWorldTransform (Variables|Default|GetFirePoint)) "Undefined" "MultiplyWithRoot" 0 0))