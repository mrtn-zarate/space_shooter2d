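; BP_BaseEnemy is a space shooter enemy that flies along its initial forward vector and self-destroys after a fixed lifetime.
; Tick drives Move and accumulates a timer that calls Fire to spawn Ammo at FirePoint with the enemy's rotation.
; Overlapping a Player-tagged actor calls OnEnemyDestroy, plays explosion effects and destroys the enemy after a short delay.
; The player-ammo cast and Destroyed_Event binding are unconnected, so neither runs.
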(event Custom|Destroyed_Event
  (Utilities|FlowControl|Delay 0.2)
  (Actor|DestroyActor))

(event EventBeginPlay
  (Variables|Default|SetMovementVector (Transformation|GetActorForwardVector))
  (Utilities|FlowControl|Delay 2e+01)
  (Actor|DestroyActor))

(event Collision|EventActorBeginOverlap
  (params (OtherActor :type Actor%20Object%20Reference))
  (if (Utilities|Array|ContainsItem (Variables|/Script/Engine.Actor|GetTags OtherActor) "Player")
    (Default|CallOnEnemyDestroy)
    (Utilities|Casting|CastTogamemodebase (Game|GetGameMode))
    (Effects|SpawnEmitteratLocation "/Game/StarterContent/Particles/P_Explosion.P_Explosion" (Transformation|GetActorLocation))
    (Audio|SpawnSound2D "/Game/00_Space_shooter/Sounds/distant-explosion.distant-explosion" 1.2 1.0 0.0 0)
    (Utilities|FlowControl|Delay 0.2)
    (Actor|DestroyActor)))

(event EventTick
  (params (DeltaSeconds :type Float%20%28single-precision%29))
  (CallFunction|Move DeltaSeconds)
  (bind _output_get (Variables|Default|SetShootCurrentTime (+ DeltaSeconds (Variables|Default|GetShootCurrentTime))))
  (if (> _output_get (Variables|Default|GetDelayShoot))
    (Variables|Default|SetShootCurrentTime 0.0)
    (CallFunction|Fire)))

(fn ConstructionScript)

(fn Move
  (params (DeltaTime :type Float%20%28double-precision%29))
  (Transformation|SetActorLocation (+ (Transformation|GetActorLocation) (* (* DeltaTime (Variables|Default|GetSpeed)) (Variables|Default|GetMovementVector))) false false))

(fn Fire
  (bind _returnvalue (Game|SpawnActorfromClass (Variables|Default|GetAmmo) (Transformation|GetWorldTransform (Variables|Default|GetFirePoint)) "Undefined" "MultiplyWithRoot" 0 0))
  (Transformation|SetActorRotation _returnvalue (Transformation|GetActorRotation)))